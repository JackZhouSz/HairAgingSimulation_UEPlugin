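; Actor component that simulates hair aging over time by animating an age value and hair thinning.
; Each tick, UpdateParams accumulates elapsed time and linearly interpolates both values from initial to final over AnimDuration.
; Age goes to the AgingSimulationParam material parameter collection, while thinning scales root and tip in every hair group's geometry settings.
; It edits the groom asset's settings directly and reassigns the asset within the loop every frame.
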(event `self.ReceiveBeginPlay`)

(event `self.ReceiveTick`
  (params (DeltaSeconds :type "Float (single-precision)"))
  (bind _hairgroom (`self.HairGroom`))
  (bind _groomasset (`GroomComponent.GroomAsset` _hairgroom))
  (bind _hairgroupsrendering (`GroomAsset.HairGroupsRendering` _groomasset))
  (bind (_age _thinning) (`self.UpdateParams` DeltaSeconds))
  (`KismetMaterialLibrary.SetScalarParameterValue` "/HairAging/AgingSimulationParam.AgingSimulationParam" "Age" _age)
  (for (_ _array_index) _hairgroupsrendering
    (`HairAgingComponent.setHairGeometrySettings` (`|GetArrayItem` _hairgroupsrendering _array_index) (make `HairGeometrySettings` 0.01 _thinning _thinning))
    (`GroomComponent.SetGroomAsset` _hairgroom _groomasset)))

(fn `UpdateParams`
  (params (DeltaSeconds :type "Float (double-precision)"))
  (returns (Age :type "Float (double-precision)") (Thinning :type "Float (double-precision)"))
  (bind _returnvalue (+ DeltaSeconds (`self.Duration`)))
  (bind _returnvalue_2 (`KismetMathLibrary.FMin` (/ _returnvalue (`self.Anim_Duration`)) 1.0))
  (set `self.Duration` _returnvalue)
  (return (`|EaseFunction` "Linear" _returnvalue_2 (`self.InitAge`) (`self.FinalAge`)) (`|EaseFunction` "Linear" _returnvalue_2 (`self.InitThinning`) (`self.FinalThinning`))))